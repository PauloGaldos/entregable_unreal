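; Door blueprint that opens when the player interacts with it after all collectables in the game mode's second counter are gathered.
; A box trigger enables input only while the player overlaps it.
; On Interact, a zero CollectablesLeft2 on playerGameMode plays a sound and a timeline lerps the mesh downward.
; Otherwise, it adds a collectable widget to the viewport.
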(event `InputAction|Interact`
  (params (Key :type "Key Structure"))
  (:`Pressed`
    (bind _asbp_first_person_game_mode (cast `/Game/FirstPerson/Blueprints/playerGameMode` (`GameplayStatics.GetGameMode`)))
    (if (== (`/Game/FirstPerson/Blueprints/playerGameMode.Collectables Left2` _asbp_first_person_game_mode) 0)
      (`GameplayStatics.SpawnSoundAttached` "/Game/puerta/punch-a-rock-161647.punch-a-rock-161647" (`self.StaticMesh`) "None" (0.0 0.0 0.0) (struct) "KeepRelativeOffset" false 1.0 1.0 0.0 null null)
      (bind (_direction _newtrack_0) (`Timeline|Timeline` :!via `PlayFromStart`)
        (:`Update`
          (`SceneComponent.K2_SetRelativeLocation` (`self.StaticMesh`) (`KismetMathLibrary.MakeVector` 0.0 0.0 (`KismetMathLibrary.Lerp` 0.0 -700.0 _newtrack_0)) false false)))
      (else
        (bind _returnvalue (`|CreateWidget` "/Game/llaves/CollectableWidget.CollectableWidget_C"))
        (`UserWidget.AddToViewport` _returnvalue 0)))))

(event `self.Box.OnComponentBeginOverlap`
  (params (OverlappedComponent :type "PrimitiveComponent Object Reference") (OtherActor :type "Actor Object Reference") (OtherComp :type "PrimitiveComponent Object Reference") (OtherBodyIndex :type Integer) (bFromSweep :type Boolean) (SweepResult :type "HitResult Structure (by ref)"))
  (cast `/Game/FirstPerson/Blueprints/player` OtherActor)
  (`self.EnableInput` (`GameplayStatics.GetPlayerController` 0)))

(event `self.Box.OnComponentEndOverlap`
  (params (OverlappedComponent :type "PrimitiveComponent Object Reference") (OtherActor :type "Actor Object Reference") (OtherComp :type "PrimitiveComponent Object Reference") (OtherBodyIndex :type Integer))
  (cast `/Game/FirstPerson/Blueprints/player` OtherActor)
  (`self.DisableInput` (`GameplayStatics.GetPlayerController` 0)))

(fn `UserConstructionScript`)