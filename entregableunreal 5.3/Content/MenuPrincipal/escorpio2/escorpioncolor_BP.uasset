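; Scorpion AI character Blueprint that wanders the level and flees when its AI Perception senses a stimulus.
; A DecideNextEvent loop chooses between slower RandomRoam and faster RunAway, each moving to a random reachable point via AIMoveTo.
; Roaming pauses briefly at random between moves, while perception updates skip the delay.
; A completed flee clears ShouldRun and resumes roaming; failed moves have no handler to continue the loop.
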(event `self.ReceiveBeginPlay`
  (`self.Decide Next Event` false))

(event `Decide Next Event`
  (params (`Skip Delay` :type Boolean))
  (if (not `Skip Delay`)
    (`KismetSystemLibrary.Delay` (`KismetMathLibrary.Conv_IntToDouble` (`KismetMathLibrary.RandomIntegerInRange` 1 5))))
  (if (`self.ShouldRun`)
    (`self.Run Away`)
    (else
      (`self.Random Roam`))))

(event `Random Roam`
  (set `CharacterMovementComponent.MaxWalkSpeed` 900.0 (`self.CharacterMovement`))
  (`|AIMoveTo` self (`NavigationSystemV1.K2_GetRandomReachablePointInRadius` (`self.K2_GetActorLocation`) 90000000.0 null null) null
    (:`OnSuccess`
      (`self.Decide Next Event` false))))

(event `Run Away`
  (set `CharacterMovementComponent.MaxWalkSpeed` 1800.0 (`self.CharacterMovement`))
  (`|AIMoveTo` self (`NavigationSystemV1.K2_GetRandomReachablePointInRadius` (`self.K2_GetActorLocation`) (`KismetMathLibrary.RandomFloatInRange` 100.0 90000000.0) null null) null
    (:`OnSuccess`
      (set `self.ShouldRun` false)
      (`self.Decide Next Event` true))))

(event `self.AIPerception.OnTargetPerceptionUpdated`
  (params (Actor :type "Actor Object Reference") (Stimulus :type "AIStimulus Structure"))
  (if (not (`self.ShouldRun`))
    (set `self.ShouldRun` (`.bSuccessfullySensed` (break `AIStimulus` Stimulus)))
    (`self.Decide Next Event` true)))

(fn `UserConstructionScript`)